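; BP_Enemy is an enemy actor that moves toward the player across the XY plane.
; BeginPlay caches GameInstance_Main and takes the player reference and enemy speed from it.
; Tick applies an unswept local offset from the world-space vector to the player, minus DistanceToStop, with Z zeroed.
; That vector is not normalized, so movement speed scales with distance.
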(event `self.ReceiveBeginPlay`
  (bind _asgame_instance_main (cast `/Game/Blueprints/Generic/GameInstance_Main` (`GameplayStatics.GetGameInstance`)))
  (set `self.GameInstance` _asgame_instance_main)
  (`self.Initialize`))

(event `Initialize`
  (bind _gameinstance (`self.GameInstance`))
  (set `self.Player` (`/Game/Blueprints/Generic/GameInstance_Main.GetPlayer` _gameinstance))
  (set `self.EnemySpeed` (`/Game/Blueprints/Generic/GameInstance_Main.EnemySpeed` _gameinstance)))

(event `self.ReceiveTick`
  (params (DeltaSeconds :type "Float (single-precision)"))
  (`self.K2_AddActorLocalOffset` (* (`self.Get Direction To Player`) (* DeltaSeconds (`self.EnemySpeed`)))))

(fn `Get Direction To Player`
  (returns (ReturnValue :type "Vector Structure"))
  (locals (`Distance To Stop` :type "Float (double-precision)" :default 100.0))
  (return (* (1.0 1.0 0.0) (- (- (`self.K2_GetActorLocation` (`self.Player`)) (`self.K2_GetActorLocation`)) (`local.Distance To Stop`)))))

(fn `UserConstructionScript`)