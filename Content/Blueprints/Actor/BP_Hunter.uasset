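; BP_Hunter is an enemy Character that chases the player and deals damage when its hit collision overlaps them.
; On BeginPlay it creates a W_Enemy widget, takes the player and speed from GameInstance_Main, then loops AIMoveTo on success, a stand-in for a planned behaviour tree.
; Incoming damage reveals health and destroys the hunter at zero.
; LookedAt also reveals health, while Feed applies small damage to the hunter itself.
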(event `self.ReceiveBeginPlay`
  ;[1 1 1] Initialization
  (bind _returnvalue (`|CreateWidget` "/Game/Blueprints/Widgets/W_Enemy.W_Enemy_C" null self))
  (bind _output_get (set `self.ActiveWidget` _returnvalue))
  (`WidgetComponent.SetWidget` (`self.Widget`) _output_get)
  (bind _asgame_instance_main (cast `/Game/Blueprints/GameInstance_Main` (`GameplayStatics.GetGameInstance`)))
  (set `self.GameInstance` _asgame_instance_main)
  (`self.Setup`)
  (`self.Follow Player`))

(event `Follow Player`
  ;[1 1 1] Move to player (Will add later to behaviour tree)
  (`|AIMoveTo` self (0.0 0.0 0.0) (`self.Player`) (`self.StoppingDistance`) :!label _label
    (:`OnSuccess`
      (goto _label))))

(event `LookedAt`
  (set `self.ShowHealth` true))

(event `self.Hit Collision.OnComponentBeginOverlap`
  (params (OverlappedComponent :type "PrimitiveComponent Object Reference") (OtherActor :type "Actor Object Reference") (OtherComp :type "PrimitiveComponent Object Reference") (OtherBodyIndex :type Integer) (bFromSweep :type Boolean) (SweepResult :type "HitResult Structure (by ref)"))
  ;[1 1 1] Damage player
  (if (== OtherActor "/Game/Blueprints/Actor/BP_Player.BP_Player")
    ;;[1 1 1] Change this later to "state for attacking player"
    (`GameplayStatics.ApplyDamage` OtherActor 25.0)))

(event `self.ReceiveAnyDamage`
  (params (Damage :type "Float (single-precision)") (DamageType :type "DamageType Object Reference") (InstigatedBy :type "Controller Object Reference") (DamageCauser :type "Actor Object Reference"))
  ;[1 1 1] Enemy Taking Damage
  (if (<= (`self.Health`) 0.0)
    (`self.K2_DestroyActor`)
    (else
      (bind _output_get (set `self.ShowHealth` true))
      (if _output_get
        (`KismetSystemLibrary.PrintString` "Enemy Took damage")
        (set `self.Health` (- (`self.Health`) Damage))
        (if (<= (`self.Health`) 0.0)
          (`self.K2_DestroyActor`))))))

(event `/Game/Blueprints/BPI_Feeding.Feed`
  ;[1 1 1] Enemy Taking Damage
  (`GameplayStatics.ApplyDamage` self 0.3)
  (`KismetSystemLibrary.PrintString` "Feeding"))

(fn `Get Direction To Player`
  (returns (ReturnValue :type "Vector Structure"))
  (locals (`Distance To Stop` :type "Float (double-precision)" :default 100.0))
  (return (* (1.0 1.0 0.0) (- (- (`self.K2_GetActorLocation` (`self.Player`)) (`self.K2_GetActorLocation`)) (`local.Distance To Stop`)))))

(fn `Setup`
  (bind _gameinstance (`self.GameInstance`))
  (set `self.Player` (`/Game/Blueprints/GameInstance_Main.GetPlayer` _gameinstance))
  (bind _output_get (set `self.EnemySpeed` (`/Game/Blueprints/GameInstance_Main.EnemySpeed` _gameinstance)))
  (set `CharacterMovementComponent.MaxWalkSpeed` _output_get (`self.CharacterMovement`)))

(fn `UserConstructionScript`)