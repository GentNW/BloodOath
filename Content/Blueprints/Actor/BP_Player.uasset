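; Player character Blueprint with mouse look, movement, stamina-limited sprint and jump, health, and combat against BP_Hunter.
; BeginPlay takes speed from GameInstance_Main and adds the W_Player HUD.
; Left click punches hunters overlapping PunchZone, or while right-click aiming spends Blood and fires a camera line trace every Tick until released.
; Tick also drains or regenerates stamina through a macro, and a timeline zooms FOV for sprinting.
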(event `self.ReceiveBeginPlay`
  (bind _returnvalue_roll (`KismetMathLibrary.BreakRotator` (`SceneComponent.K2_GetComponentRotation` (`self.Camera`))))
  (bind _asgame_instance_main (cast `/Game/Blueprints/Generic/GameInstance_Main` (`GameplayStatics.GetGameInstance`)))
  (bind _output_get (set `self.GameInstance` _asgame_instance_main))
  (set `self.Speed` (`/Game/Blueprints/Generic/GameInstance_Main.PlayerSpeed` _output_get))
  (`self.Reset Speed`)
  (`self.Set Widget`)
  (set `self.TiltRotation` (`KismetMathLibrary.MakeRotator` (+ _returnvalue_roll (`self.Angle`)))))

(event `self.ReceiveActorBeginOverlap`
  (params (OtherActor :type "Actor Object Reference")))

(event `Event PunchZoneOverlap`
  (params (NewParam :type Boolean)))

(event `self.ReceiveTick`
  (params (DeltaSeconds :type "Float (single-precision)"))
  (bind _camera (`self.Camera`))
  (bind _returnvalue (`SceneComponent.K2_GetComponentLocation` _camera))
  (`self.Stamina usage`
    (:`Continue`
      _)
    (:`Stamina Is Out`
      (`self.FOV Zoom` false)))
  (if (`self.IsFiring`)
    (bind _outhit (`KismetSystemLibrary.LineTraceSingle` :`Start` _returnvalue :`End` (+ _returnvalue (* (`KismetMathLibrary.GetForwardVector` (`SceneComponent.K2_GetComponentRotation` _camera)) 1500.0)) :`TraceChannel` "TraceTypeQuery1" :`DrawDebugType` "ForOneFrame"))
    (bind _asbp_hunter (cast `/Game/Blueprints/Actor/BP_Hunter` (`.HitActor` (`GameplayStatics.BreakHitResult` _outhit))))
    (`GameplayStatics.ApplyDamage` _asbp_hunter)))

(event `InputAxisKey|MouseX`
  (params (AxisValue :type "Float (single-precision)"))
  ;[1 1 1] Camera Movement
  (`self.Camera controls` AxisValue (stale `InputAxisKey|MouseY` AxisValue) :!label _label))

(event `InputAxisKey|MouseY`
  (params (AxisValue :type "Float (single-precision)"))
  ;[1 1 1] Camera Movement
  (goto _label :!via `execute2`))

(event `InputAxis|Horizontal`
  (params (AxisValue :type "Float (single-precision)"))
  ;[1 1 1] Player Movement
  (`self.Movement Controls` AxisValue (stale `InputAxis|Vertical` AxisValue) :!label _label_2))

(event `InputAxis|Vertical`
  (params (AxisValue :type "Float (single-precision)"))
  ;[1 1 1] Player Movement
  (goto _label_2 :!via `Vetical Input`))

(event `Key|RightMouseButton`
  (params (Key :type "Key Structure"))
  (:`Pressed`
    (set `self.IsAiming` true)
    (if (`self.Firing&Aiming`) :!label _label_3
      (`KismetSystemLibrary.PrintString` "FIre Blood")
      (set `self.Blood` (- (`self.Blood`) 10.0))
      (else
        (`self.Punching`))))
  (:`Released`
    (set `self.IsAiming` false)))

(event `Key|D`
  (params (Key :type "Key Structure")))

(event `Key|LeftShift`
  (params (Key :type "Key Structure"))
  ;[1 1 1] Sprint Trigger
  (:`Pressed`
    (`self.Start Sprinting`)
    (`self.FOV Zoom` true))
  (:`Released`
    (`self.Stop Sprinting`)
    (`self.FOV Zoom` false)))

(event `Key|A`
  (params (Key :type "Key Structure")))

(event `Key|LeftMouseButton`
  (params (Key :type "Key Structure"))
  (:`Pressed`
    (`self.IsMeleeOrRanged`)
    (goto _label_3))
  (:`Released`
    (`self.ClearingFire&Punch`)))

(event `FOV Zoom`
  (params (`Play forward ?` :type Boolean))
  ;[1 1 1] Sprint Trigger
  (if `Play forward ?`
    (bind (_direction _zooming) (`Timeline|Zoom` :!label _label_4)
      (:`Update`
        (`CameraComponent.SetFieldOfView` (`self.Camera`) _zooming)))
    (else
      (goto _label_4 :!via `Reverse`))))

(event `self.ReceiveAnyDamage`
  (params (Damage :type "Float (single-precision)") (DamageType :type "DamageType Object Reference") (InstigatedBy :type "Controller Object Reference") (DamageCauser :type "Actor Object Reference"))
  ;[1 1 1] Damage
  (`self.Apply Damage To Player` Damage))

(event `InputAction|Jump`
  (params (Key :type "Key Structure"))
  ;[1 1 1] Jumping
  (:`Pressed`
    (`self.Player Jump`)))

(fn `Apply Damage To Player`
  (params (`Damage Taken` :type "Float (double-precision)"))
  (set `self.Health` (- (`self.Health`) `Damage Taken`)))

(fn `ClearingFire&Punch`
  (set `self.IsFiring` false)
  (set `self.IsPunching` false))

(fn `Consume Running Stamina`
  (bind _output_get (set `self.Stamina` (`KismetMathLibrary.FClamp` (- (`self.Stamina`) (* (`GameplayStatics.GetWorldDeltaSeconds`) 20.0)) 0.0 100.0)))
  (if (== _output_get 0.0)
    (`self.Reset Speed`)
    (set `self.IsSprinting` false)
    (`KismetSystemLibrary.PrintString` "Finished Stamina")))

(fn `Firing&Aiming`
  (returns (Result :type Boolean))
  (return (and (`self.IsAiming`) (`self.IsFiring`))))

(fn `Is Player Moving`
  (returns (`Is Moving ?` :type Boolean))
  (return (> (`KismetMathLibrary.VSize` (`self.GetVelocity` (`GameplayStatics.GetPlayerCharacter` 0))) 0.0)))

(fn `IsMeleeOrRanged`
  (if (`self.IsAiming`)
    (set `self.IsFiring` true)
    (else
      (set `self.IsPunching` true))))

(fn `Player Jump`
  (locals (JumpStamina :type "Float (double-precision)" :default 30.0))
  (if (> (`self.Stamina`) (`local.JumpStamina`))
    (`self.Jump`)
    (set `self.Stamina` (- (`self.Stamina`) (`local.JumpStamina`)))))

(fn `Punching`
  (bind _overlappingactors (`PrimitiveComponent.GetOverlappingActors` (`self.Punch_Zone`) "/Game/Blueprints/Actor/BP_Hunter.BP_Hunter_C"))
  (if (`self.IsPunching`)
    (for _array_element _overlappingactors
      (if (not (== (`KismetArrayLibrary.Array_Length` _overlappingactors) 0))
        (`GameplayStatics.ApplyDamage` _array_element)
        (`KismetSystemLibrary.PrintString` "Pissing")))))

(fn `Regenerate Stamina`
  (set `self.Stamina` (`KismetMathLibrary.FClamp` (+ (`self.Stamina`) (* (`GameplayStatics.GetWorldDeltaSeconds`) 10.0)) 0.0 100.0)))

(fn `Reset Speed`
  (set `CharacterMovementComponent.MaxWalkSpeed` (`self.Speed`) (`self.CharacterMovement`)))

(fn `Set Widget`
  (bind _returnvalue (`|CreateWidget` "/Game/Blueprints/Widgets/W_Player.W_Player_C" null self))
  (`UserWidget.AddToViewport` _returnvalue 0))

(fn `Start Sprinting`
  (if (`self.Is Player Moving`)
    (if (> (`self.Stamina`) 0.1)
      (set `self.IsSprinting` true)
      (set `CharacterMovementComponent.MaxWalkSpeed` (* (`self.Speed`) 2.0) (`self.CharacterMovement`)))))

(fn `Stop Sprinting`
  (set `self.IsSprinting` false)
  (`self.Reset Speed`))

(fn `UserConstructionScript`)