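; BP_MainGameMode is the game mode that decides which NPC spawner may spawn, based on player position and facing.
; BeginPlay caches the player and all BP_NPCSpawner actors, which Tick passes to GetPlayerDirection through a zero-second Delay.
; A distance and dot-product test selects the first nearby spawner behind the player's facing and calls StartSpawn.
; Failing spawners checked before it are marked unspawnable, while the break leaves later ones untouched.
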(event `self.ReceiveBeginPlay`
  (bind _asbp_player (cast `/Game/Blueprints/Actor/BP_Player` (`GameplayStatics.GetPlayerPawn` 0)))
  (set `self.Player` _asbp_player)
  (bind _outactors (`GameplayStatics.GetAllActorsOfClass` "/Game/Blueprints/Actor/BP_NPCSpawner.BP_NPCSpawner_C"))
  (set `self.Spawners` _outactors))

(event `self.ReceiveTick`
  (params (DeltaSeconds :type "Float (single-precision)"))
  (`KismetSystemLibrary.Delay` 0.0)
  (`self.GetPlayerDirection` (`self.Spawners`)))

(fn `GetPlayerDirection`
  (params (Spawners :type "Array of Actor Object Reference"))
  (bind _spawner (`self.Spawner`))
  (bind _player (`self.Player`))
  (bind _returnvalue (`self.K2_GetActorLocation` (`self.Spawner`)))
  (bind _returnvalue_2 (`self.K2_GetActorLocation` _player))
  (for _array_element Spawners
    (bind _asbp_npcspawner (cast `/Game/Blueprints/Actor/BP_NPCSpawner` _array_element))
    (set `self.Spawner` _asbp_npcspawner)
    (bind _output_get (set `self.SpawnerToPlayer` (- _returnvalue_2 _returnvalue)))
    (if (and (< (`KismetMathLibrary.Vector_Distance` _returnvalue_2 _returnvalue) (`self.DistanceToSpawn`)) (`KismetMathLibrary.InRange_FloatFloat` (`KismetMathLibrary.Dot_VectorVector` (`KismetMathLibrary.Normal` _output_get) (`KismetMathLibrary.Normal` (`self.GetActorForwardVector` _player))) 0.7 1.0))
      (set `/Game/Blueprints/Actor/BP_NPCSpawner.IsSpawnable` true _spawner)
      (`/Game/Blueprints/Actor/BP_NPCSpawner.StartSpawn` _spawner)
      (break)
      (else
        (set `/Game/Blueprints/Actor/BP_NPCSpawner.IsSpawnable` false _spawner)))))

(fn `UserConstructionScript`)