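; BP_Player is the player pawn Blueprint, handling mouse look and axis-driven movement.
; MouseX and inverted MouseY feed controller yaw and pitch, then both reset player 0's control rotation roll to zero.
; Horizontal and Vertical axes add movement input along the SpringArm's right and forward vectors, with the forward vector not flattened to the ground plane.
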(event `self.ReceiveTick`
  (params (DeltaSeconds :type "Float (single-precision)")))

(event `InputAxisKey|MouseX`
  (params (AxisValue :type "Float (single-precision)"))
  (bind _returnvalue (`GameplayStatics.GetPlayerController` 0))
  (bind (_returnvalue_roll _returnvalue_pitch _returnvalue_yaw) (`KismetMathLibrary.BreakRotator` (`Controller.GetControlRotation` _returnvalue)))
  (`self.AddControllerYawInput` AxisValue)
  (`Controller.SetControlRotation` _returnvalue (`KismetMathLibrary.MakeRotator` 0.0 _returnvalue_pitch _returnvalue_yaw) :!label _label))

(event `InputAxisKey|MouseY`
  (params (AxisValue :type "Float (single-precision)"))
  (`self.AddControllerPitchInput` (* -1 AxisValue))
  (goto _label))

(event `InputAxis|Horizontal`
  (params (AxisValue :type "Float (single-precision)"))
  (`self.AddMovementInput` (`SceneComponent.GetRightVector` (`self.SpringArm`)) AxisValue))

(event `InputAxis|Vertical`
  (params (AxisValue :type "Float (single-precision)"))
  (`self.AddMovementInput` (`SceneComponent.GetForwardVector` (`self.SpringArm`)) AxisValue))

(fn `UserConstructionScript`)