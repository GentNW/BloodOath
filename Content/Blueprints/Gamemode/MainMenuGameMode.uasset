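; Game mode Blueprint with disconnected logic for choosing the default pawn by level.
; IsPlayable returns true when the current level name differs from MainMenuLvl.
; Two unreachable chains use that check to set DefaultPawnClass to BP_Player or BP_MenuView, then call ResetLevel.
; BeginPlay, Tick and the construction script are empty, so none of this switching runs.
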(event `self.ReceiveBeginPlay`)

(event `self.ReceiveTick`
  (params (DeltaSeconds :type "Float (single-precision)")))

(fn `IsPlayable`
  (returns (ReturnValue :type Boolean))
  (bind _returnvalue (`GameplayStatics.GetCurrentLevelName` true))
  (return (`KismetStringLibrary.NotEqual_StrStr` _returnvalue (`self.MainMenuLvl`))))

(fn `UserConstructionScript`)