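; Game instance Blueprint that provides global helpers for player access and on-screen dialogue.
; GetPlayer returns the first player pawn cast to BP_Player.
; StartDialogue lazily creates a single W_Dialogue widget, adds it to the viewport, caches it and returns the current DialogueLine.
; ChangeDialogueText updates the stored DialogueLine only while that widget is valid, without calling the widget directly.
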(fn `Change Dialogue Text`
  (params (Text :type Text))
  (`/Engine/EditorBlueprintResources/StandardMacros.IsValid` (`self.Dialogue Widget`)
    (:`Is Valid`
      (set `self.Dialogue Line` Text))))

(fn `GetPlayer`
  (returns (Player :type "/Game/Blueprints/Actor/BP_Player Object Reference"))
  (bind _asbp_player (cast `/Game/Blueprints/Actor/BP_Player` (`GameplayStatics.GetPlayerPawn` 0)))
  (return _asbp_player))

(fn `Start Dialogue`
  (returns (Dialogue :type Text))
  (`/Engine/EditorBlueprintResources/StandardMacros.IsValid` (`self.Dialogue Widget`)
    (:`Is Valid`
      _)
    (:`Is Not Valid`
      (bind _returnvalue (`|CreateWidget` "/Game/Blueprints/Widgets/W_Dialogue.W_Dialogue_C" null self))
      (`UserWidget.AddToViewport` _returnvalue 0)
      (set `self.Dialogue Widget` _returnvalue)))
  (return (`self.Dialogue Line`)))